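; BP_TrafficCar is a looping ambient traffic car that stops for obstacles and stop lights.
; A Timeline lerps it from its spawn point to the Cube's location, then teleports it back with a random skeletal mesh and restarts.
; A repeating timer box-traces ahead: a BP_StopLight hit halts it, any other hit also sounds the horn, and a clear path resumes movement.
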(event `self.ReceiveBeginPlay`
  (bind _returnvalue (`KismetSystemLibrary.K2_SetTimerDelegate` (delegate `EventTrace`) 0.2 true))
  (set `self.Timer` _returnvalue)
  (bind _asbp_player_granny (cast `/Game/Game/Blueprints/Player/BP_Player_Granny` (`GameplayStatics.GetPlayerCharacter` 0)))
  (set `self.PlayerRef` _asbp_player_granny)
  (set `self.EndPosition` (`SceneComponent.K2_GetComponentLocation` (`self.Cube`)))
  (set `self.StartPosition` (`self.K2_GetActorLocation`))
  (`self.SetAnyCarsForArray`))

(event `EventTrace`
  (bind _scene (`self.Scene`))
  (bind _car_horn_cue (`self.Car_Horn_Cue`))
  (bind _returnvalue (`SceneComponent.K2_GetComponentLocation` _scene))
  (bind (_outhit _returnvalue_2) (`KismetSystemLibrary.BoxTraceSingle` :`Start` _returnvalue :`End` (+ (* (`SceneComponent.GetForwardVector` _scene) (800.0 0.0 0.0)) _returnvalue) :`HalfSize` (120.0 300.0 50.0) :`TraceChannel` "TraceTypeQuery3" :`DrawTime` 0.2))
  (if _returnvalue_2
    (cast `/Game/Game/Blueprints/Environment/Interact/BP_StopLight` (`.HitActor` (`GameplayStatics.BreakHitResult` _outhit))
      (:`then`
        (bind (_direction _newtrack_0) (`Timeline|Timeline` :`NewTime` (`self.CurrentTime`) :!via `Stop` :!label _label)
          (:`Update`
            (set `self.CurrentTime` _newtrack_0)
            (bind _returnvalue_3 (`KismetMathLibrary.VLerp` (`self.StartPosition`) (`self.EndPosition`) _newtrack_0))
            (set `self.CurrentPosition` _returnvalue_3)
            (`self.K2_SetActorLocation` _returnvalue_3)
            (if (`KismetMathLibrary.EqualExactly_VectorVector` (`self.CurrentPosition`) (`self.EndPosition`))
              (`self.K2_SetActorLocation` (`self.StartPosition`) false true)
              (`self.SetAnyCarsForArray`)
              (set `self.CurrentTime` 0.0)
              (goto _label :!via `PlayFromStart`)))))
      (:`CastFailed`
        (`AudioComponent.Play` _car_horn_cue 0.0)
        (goto _label :!via `Stop`)))
    (else
      (`AudioComponent.Stop` _car_horn_cue)
      (goto _label))))

(fn `SetAnyCarsForArray`
  (bind _output_get (set `self.CurrentCar` (`KismetArrayLibrary.Array_Random` (`self.VarCars`))))
  (`SkeletalMeshComponent.SetSkeletalMeshAsset` (`self.SkeletalMesh`) _output_get))

(fn `UserConstructionScript`)